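; Player character with directional flipbook sprites that moves on two axes, dashes, toggles an electric vision and talks to NPCs.
; Dash teleports along the input direction, leaving a sprite afterimage and a beam that follows the player until a timeline ends.
; Tick picks the flipbook from last direction and state, and snaps height to the ground by line trace.
; ElecVision fades a material parameter collection and vignette, while capsule overlap stores the NPC for Interact, which blocks input.
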(event OnComponentBeginOverlap(CapsuleComponent)
  (params (OverlappedComponent :type Primitive%20Component%20Object%20Reference) (OtherActor :type Actor%20Object%20Reference) (OtherComp :type Primitive%20Component%20Object%20Reference) (OtherBodyIndex :type Integer) (bFromSweep :type Boolean) (SweepResult :type Hit%20Result%20Structure%20%28by%20ref%29))
  ;[1 1 1] Overlaps
  (bind _asbp_npc (Utilities|Casting|CastToBP_NPC OtherActor))
  (Variables|Default|SetRefNPC _asbp_npc))

(event OnComponentEndOverlap(CapsuleComponent)
  (params (OverlappedComponent :type Primitive%20Component%20Object%20Reference) (OtherActor :type Actor%20Object%20Reference) (OtherComp :type Primitive%20Component%20Object%20Reference) (OtherBodyIndex :type Integer))
  ;[1 1 1] Overlaps
  (Variables|Default|SetRefNPC 0))

(event EventTick
  (params (DeltaSeconds :type Float%20%28single-precision%29))
  ;[1 1 1] Tick
  (CallFunction|SetFlipbookDir)
  (CallFunction|CalculateGround))

(event Input|ActionEvents|InputActionElecVision
  (params (Key :type Key%20Structure :default "None"))
  ;[1 1 1] ElecVision
  (:Pressed
    (Utilities|FlowControl|FlipFlop
      (:A
        (bind _blendvalue (Timeline|BlendWeight Play)
          (:Update
            (Rendering|Material|SetScalarParameterValue "/Game/MPC_ElecVision.MPC_ElecVision" "Alpha" _blendvalue :!class /Script/Engine.KismetMaterialLibrary)
            (Utilities|Struct|SetmembersinPostProcessSettings (Variables|/Script/Engine.PostProcessComponent|GetSettings (Variables|Default|GetPP_ElecVision)) _blendvalue))))
      (:B
        (Timeline|BlendWeight Reverse)))))

(event Input|ActionEvents|InputActionInteract
  (params (Key :type Key%20Structure :default "None"))
  ;[1 1 1] Interaction
  (:Pressed
    (if (not (Variables|Default|GetBlockInput?))
      (Utilities|IsValid (Variables|Default|GetRefNPC)
        (:Is%20Valid
          (Default|LaunchDialogue (Variables|Default|GetRefNPC))
          (Variables|Default|SetBlockInput? true))))))

(event Input|ActionEvents|InputActionDash
  (params (Key :type Key%20Structure :default "None"))
  (bind _returnvalue (Transformation|GetActorLocation))
  (bind _returnvalue_2 (Input|AxisValues|GetRightAxis))
  (bind _returnvalue_3 (Input|AxisValues|GetUpAxis))
  (bind _returnvalue_4 (Math|Vector|MakeVector _returnvalue_3 _returnvalue_2 0.0))
  (bind _returnvalue_5 (Math|Vector|Normalize _returnvalue_4))
  (bind _returnvalue_6 (* _returnvalue_5 -1e+02))
  (bind _returnvalue_7 (+ _returnvalue_6 _returnvalue))
  ;[1 1 1] Dash Action
  (:Pressed
    (if (and (not (Variables|Default|GetDashing?)) (or (!= (Input|AxisValues|GetUpAxis) 0.0) (!= (Input|AxisValues|GetRightAxis) 0.0)))
      (bind _returnvalue_8 (Game|SpawnActorfromClass "/Game/Blueprints/BP_DashFade.BP_DashFade_C" (Math|Transform|MakeTransform (.location (Transformation|GetActorTransform)) "0,-90.000000, 0" (Transformation|GetWorldScale (Variables|Default|GetSprite))) "Undefined" 0 0))
      (Rendering|Components|Sprite|SetSprite (Variables|/Script/Paper2D.PaperSpriteActor|GetRenderComponent _returnvalue_8) (Class|PaperFlipbook|GetSpriteatTime (Class|PaperFlipbookComponent|GetFlipbook (Variables|Default|GetSprite)) 0.0 false))
      (Variables|Default|SetDashing? true)
      (Development|PrintString (Utilities|String|ToString(Vector) _returnvalue_7))
      (Transformation|SetActorLocation _returnvalue_7 false true)
      (bind _returnvalue_9 (Effects|SpawnEmitteratLocation "/Game/MyParticleSystems/Beam/P_Beam.P_Beam" "0, 0, 0"))
      (Class|ParticleSystemComponent|SetBeamSourcePoint _returnvalue_9 0 (Transformation|GetActorLocation _returnvalue_8))
      (Timeline|Timeline_0 PlayFromStart
        (:Update
          (Class|ParticleSystemComponent|SetBeamTargetPoint _returnvalue_9 0 (Transformation|GetActorLocation)))
        (:Finished
          (Variables|Default|SetDashing? false))))))

(event Input|AxisEvents|InputAxisUpAxis
  (params (AxisValue :type Float%20%28single-precision%29))
  ;[1 1 1] Déplacement
  (if (not (Variables|Default|GetBlockInput?))
    (Pawn|Input|AddMovementInput "-1.000000,0.000000,0.000000" AxisValue false)))

(event Input|AxisEvents|InputAxisRightAxis
  (params (AxisValue :type Float%20%28single-precision%29))
  ;[1 1 1] Déplacement
  (if (not (Variables|Default|GetBlockInput?))
    (Pawn|Input|AddMovementInput "0.000000,-1.000000, 0" AxisValue false)))

(fn ConstructionScript
  (Transformation|SetWorldRotation (Variables|Default|GetSprite) (Math|Rotator|MakeRotator (.pitch (Transformation|GetWorldRotation (Variables|Default|GetSpringArm))) 0.0 -9e+01) false false))

(fn SetFlipbookDir
  (bind _returnvalue (Transformation|GetVelocity))
  (bind _returnvalue_2 (Input|AxisValues|GetUpAxis))
  (bind _sprite (Variables|Default|GetSprite))
  (bind _returnvalue_3 (Math|Vector|VectorLength _returnvalue))
  (bind _returnvalue_4 (> _returnvalue_3 0.0))
  (if (Variables|Default|GetBlockInput?)
    (Sprite|SetFlipbook _sprite (select _returnvalue_4 (Utilities|Select :Index (Variables|Default|GetlastMoveDir) :NewEnumerator0 "/Game/Textures/Character/FB_RunUp.FB_RunUp" :NewEnumerator1 "/Game/Textures/Character/FB_RunDown.FB_RunDown" :NewEnumerator2 "/Game/Textures/Character/FB_RunLeft.FB_RunLeft" :NewEnumerator3 "/Game/Textures/Character/FB_RunRight.FB_RunRight") (Utilities|Select :Index (Variables|Default|GetlastMoveDir) :NewEnumerator0 "/Game/Textures/Character/FB_IdleUp.FB_IdleUp" :NewEnumerator1 "/Game/Textures/Character/FB_IdleDown.FB_IdleDown" :NewEnumerator2 "/Game/Textures/Character/FB_IdleLeft.FB_IdleLeft" :NewEnumerator3 "/Game/Textures/Character/FB_IdleRight.FB_IdleRight")) :!label _label)
    (else
      (if (or (!= (Input|AxisValues|GetUpAxis) 0.0) (!= (Input|AxisValues|GetRightAxis) 0.0))
        (Variables|Default|SetlastMoveDir (select (> _returnvalue_2 0.0) "NewEnumerator0" (select (< _returnvalue_2 0.0) "NewEnumerator1" (select (> (Input|AxisValues|GetRightAxis) 0.0) "NewEnumerator3" "NewEnumerator2"))))
        (if (Variables|Default|GetDashing?)
          (goto _label)
          (else
            _)))
      (Sprite|SetFlipbook _sprite (select _returnvalue_4 (Utilities|Select :Index (Variables|Default|GetlastMoveDir) :NewEnumerator0 "/Game/Textures/Character/FB_WalkUp.FB_WalkUp" :NewEnumerator1 "/Game/Textures/Character/FB_WalkDown.FB_WalkDown" :NewEnumerator2 "/Game/Textures/Character/FB_WalkLeft.FB_WalkLeft" :NewEnumerator3 "/Game/Textures/Character/FB_WalkRight.FB_WalkRight") (Utilities|Select :Index (Variables|Default|GetlastMoveDir) :NewEnumerator0 "/Game/Textures/Character/FB_IdleUp.FB_IdleUp" :NewEnumerator1 "/Game/Textures/Character/FB_IdleDown.FB_IdleDown" :NewEnumerator2 "/Game/Textures/Character/FB_IdleLeft.FB_IdleLeft" :NewEnumerator3 "/Game/Textures/Character/FB_IdleRight.FB_IdleRight"))))))

(fn CalculateGround
  (bind _returnvalue (Transformation|GetActorLocation))
  (bind _returnvalue_2 (Transformation|GetActorLocation))
  (bind _outhit (Collision|LineTraceByChannel (Math|Vector|MakeVector (.x _returnvalue_2) (.y _returnvalue_2) (+ (.z _returnvalue_2) 3e+01)) (Math|Vector|MakeVector (.x _returnvalue_2) (.y _returnvalue_2) (- (.z _returnvalue_2) 2e+02)) "TraceTypeQuery1" false 0 "ForOneFrame"))
  (Transformation|SetActorLocation (Math|Vector|MakeVector (.x _returnvalue) (.y _returnvalue) (+ (.z (.impactpoint _outhit)) (Variables|Default|GetDistFromGround))) false false))

(fn BlockInput
  (params (Block? :type Boolean))
  (if Block?
    (Variables|Default|SetBlockInput? true)
    (else
      (Variables|Default|SetBlockInput? false))))

(fn VerifySprint
  (bind _charactermovement (Variables|Character|GetCharacterMovement))
  (if (and (Variables|Default|GetDashing?) (or (> (Math|Float|Absolute(Float) (Input|AxisValues|GetUpAxis)) 0.2) (> (Math|Float|Absolute(Float) (Input|AxisValues|GetRightAxis)) 0.2)))
    (Variables|/Script/Engine.CharacterMovementComponent|SetMaxFlySpeed _charactermovement 7.5e+02)
    (else
      (Variables|/Script/Engine.CharacterMovementComponent|SetMaxFlySpeed _charactermovement 3e+02)
      (Variables|Default|SetDashing? false))))